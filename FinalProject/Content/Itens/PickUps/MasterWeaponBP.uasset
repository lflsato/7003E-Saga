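; Base weapon pickup that highlights on overlap, lets KalebeCharacter pick it up, and handles firing and reloading.
; Firing loops through a gate and retriggerable delay, paced by whether a rifle or sniper is equipped.
; Each shot line-traces from the camera, sends random damage through the TakeDamage interface, and spawns a muzzle projectile toward the hit.
; Ammo lives in ItemInfo; releasing fire on an empty clip auto-reloads from reserve with montage and sounds.
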(event `self.Sphere.OnComponentBeginOverlap`
  (params (OverlappedComponent :type "PrimitiveComponent Object Reference") (OtherActor :type "Actor Object Reference") (OtherComp :type "PrimitiveComponent Object Reference") (OtherBodyIndex :type Integer) (bFromSweep :type Boolean) (SweepResult :type "HitResult Structure (by ref)"))
  (bind _askalebe_character (cast `/Game/Kalebe/Blueprints/KalebeCharacter` OtherActor))
  (set `self.CharacterRef` _askalebe_character)
  (`self.On/OffVisibility/CustomDepth` true true)
  (set `self.CanWePick?` true)
  (`self.EnableInput` (`GameplayStatics.GetPlayerController` 0)))

(event `self.Sphere.OnComponentEndOverlap`
  (params (OverlappedComponent :type "PrimitiveComponent Object Reference") (OtherActor :type "Actor Object Reference") (OtherComp :type "PrimitiveComponent Object Reference") (OtherBodyIndex :type Integer))
  (bind _askalebe_character (cast `/Game/Kalebe/Blueprints/KalebeCharacter` OtherActor))
  (set `self.CharacterRef` _askalebe_character)
  (`self.On/OffVisibility/CustomDepth` false)
  (set `self.CanWePick?` false))

(event `InputAction|ItemIteraction`
  (params (Key :type "Key Structure"))
  (:`Pressed`
    (if (`self.CanWePick?`)
      (`/Game/Kalebe/Blueprints/KalebeCharacter.Pickup` (`self.CharacterRef`) self))))

(event `OffAll`
  (`self.On/OffVisibility/CustomDepth` false)
  (`ActorComponent.K2_DestroyComponent` (`self.Sphere`)))

(event `StartFire`
  (bind _characterref (`self.CharacterRef`))
  (bind _skeletalmesh (`self.SkeletalMesh`))
  (bind _returnvalue (`SceneComponent.GetSocketLocation` (`self.SkeletalMesh`) "MuzzleFlash"))
  (bind _followcamera (`/Game/Kalebe/Blueprints/KalebeCharacter.FollowCamera` (`self.CharacterRef`)))
  (bind _returnvalue_2 (`SceneComponent.K2_GetComponentLocation` _followcamera))
  (`|ExecutionSequence`
    (:`then_0`
      (goto _label :!via `Open`))
    (:`then_1`
      (`/Engine/EditorBlueprintResources/StandardMacros.Gate` true :!label _label
        (:`Exit`
          (`|ExecutionSequence`
            (:`then_0`
              ;[1 1 1] Verify fire frequency
              (if (`/Game/Kalebe/Blueprints/KalebeCharacter.Equip Rifle` _characterref)
                (`KismetSystemLibrary.RetriggerableDelay` 0.1)
                (goto _label)
                (elif (`/Game/Kalebe/Blueprints/KalebeCharacter.Equip Sniper` _characterref)
                  (`KismetSystemLibrary.RetriggerableDelay` 0.8)
                  (goto _label))))
            (:`then_1`
              (if (<= (`.CurrentAmmo_30_8B43CCA8494499899EBAC5A52E9121F5` (break `/Game/Itens/PickUps/ItemType` (`self.ItemInfo`))) 0)
                (`KismetSystemLibrary.PrintString` "Out of Ammos")
                (else
                  (bind (_outhit _returnvalue_3) (`KismetSystemLibrary.LineTraceSingle` _returnvalue_2 (+ _returnvalue_2 (* (`SceneComponent.GetForwardVector` _followcamera) 15000.0)) "TraceTypeQuery2"))
                  (`GameplayStatics.PlaySound2D` "/Game/MilitaryWeapSilver/Sound/Rifle/Cues/RifleA_Fire_Cue.RifleA_Fire_Cue" 1.0 1.0 0.0 null null)
                  (`Character.PlayAnimMontage` (`self.CharacterRef`) (`self.PlayFireAnim`) 1.0 "None")
                  (setmembers `/Game/Itens/PickUps/ItemType` :`StructRef` (`self.ItemInfo`) :`CurrentAmmo` (- (`.CurrentAmmo_30_8B43CCA8494499899EBAC5A52E9121F5` (break `/Game/Itens/PickUps/ItemType` (`self.ItemInfo`))) 1))
                  (bind (_bblockinghit _binitialoverlap _time _distance _location _impactpoint _normal _impactnormal _physmat _hitactor _hitcomponent _hitbonename _hititem _faceindex _tracestart _traceend) (`GameplayStatics.BreakHitResult` _outhit))
                  (if (`KismetSystemLibrary.DoesImplementInterface` _hitactor "/Game/Enemies/Monster/Blueprints/TakeDamage.TakeDamage_C")
                    (message `/Game/Enemies/Monster/Blueprints/TakeDamage.ITakeDamage` _hitactor _hitbonename (`KismetMathLibrary.RandomFloatInRange` 20.0 35.0)))
                  (`|SpawnActorFromClass` "/Game/Itens/PickUps/Projecttile_BP.Projecttile_BP_C" (`KismetMathLibrary.MakeTransform` _returnvalue (`KismetMathLibrary.FindLookAtRotation` _returnvalue (`KismetMathLibrary.SelectVector` _impactpoint _traceend _returnvalue_3))) "Undefined" "OverrideRootScale" null null)
                  (`GameplayStatics.SpawnEmitterAtLocation` "/Game/MilitaryWeapSilver/FX/P_Impact_Metal_Medium_01.P_Impact_Metal_Medium_01" _location)
                  (`GameplayStatics.SpawnEmitterAttached` "/Game/MilitaryWeapSilver/FX/P_AssaultRifle_MuzzleFlash.P_AssaultRifle_MuzzleFlash" (`self.SkeletalMesh`) "MuzzleFlash" (`SceneComponent.GetSocketLocation` _skeletalmesh "MuzzleFlash") (`SceneComponent.GetSocketRotation` _skeletalmesh "MuzzleFlash") (1.0 1.0 1.0) "KeepWorldPosition"))))))))))

(event `StopFire`
  (goto _label :!via `Close`))

(event `FirePress`
  (set `self.CanFire` true)
  (if (not (`self.IsReloading`))
    (`self.StartFire`)))

(event `FireRelease`
  (set `self.CanFire` false)
  (`self.StopFire`)
  (`self.AutoReload`))

(event `AutoReload`
  (if (== (`.CurrentAmmo_30_8B43CCA8494499899EBAC5A52E9121F5` (break `/Game/Itens/PickUps/ItemType` (`self.ItemInfo`))) 0)
    (if (== (`.MaxAmmo_31_F054BC5D47269EC4CA695EBDF480892B` (break `/Game/Itens/PickUps/ItemType` (`self.ItemInfo`))) 0)
      (`KismetSystemLibrary.PrintString` "Find Ammo")
      (else
        (set `self.IsReloading` true)
        (`self.Reloading`)
        (`KismetSystemLibrary.Delay` 2.0) ; Reload Amin Time
        (set `self.IsReloading` false)))))

(event `Reloading`
  (bind ((`ItemClass_41_89E932C2402F2CE6B811CBB923E709C0` _itemclass) (`ClipSize_40_72C2966E40FC4674620B56A55A8AC1F1` _clipsize) (`MaxAmmo_31_F054BC5D47269EC4CA695EBDF480892B` _maxammo)) (break `/Game/Itens/PickUps/ItemType` (`self.ItemInfo`)))
  (if (== (`.MaxAmmo_31_F054BC5D47269EC4CA695EBDF480892B` (break `/Game/Itens/PickUps/ItemType` (`self.ItemInfo`))) 0)
    (`KismetSystemLibrary.PrintString` "Find Ammo")
    (elif (== _clipsize _maxammo)
      (`KismetSystemLibrary.PrintString` "Full Ammo")
      (else
        (set `self.IsReloading` true)
        (if true
          (`self.WeaponReload`)
          (`KismetSystemLibrary.Delay` 2.0)
          (set `self.IsReloading` false))))))

(event `WeaponReload`
  (bind _iteminfo (`self.ItemInfo`))
  (bind _neededammo (`self.NeededAmmo`))
  (bind ((`ClipSize_40_72C2966E40FC4674620B56A55A8AC1F1` _clipsize) (`CurrentAmmo_30_8B43CCA8494499899EBAC5A52E9121F5` _currentammo)) (break `/Game/Itens/PickUps/ItemType` (`self.ItemInfo`)))
  (bind ((`MaxAmmo_31_F054BC5D47269EC4CA695EBDF480892B` _maxammo)) (break `/Game/Itens/PickUps/ItemType` (`self.ItemInfo`)))
  (bind ((`CurrentAmmo_30_8B43CCA8494499899EBAC5A52E9121F5` _currentammo_2) (`MaxAmmo_31_F054BC5D47269EC4CA695EBDF480892B` _maxammo_2)) (break `/Game/Itens/PickUps/ItemType` (`self.ItemInfo`)))
  (if (not (`self.CanFire`))
    (bind _returnvalue (`Character.PlayAnimMontage` (`self.CharacterRef`) "/Game/Kalebe/Animations/Rifle_Reload_Montage.Rifle_Reload_Montage" 1.0 "None"))
    (`KismetSystemLibrary.PrintString` "Hello" true true (struct :`G` 0.66 :`B` 1.0 :`A` 1.0) _returnvalue)
    (`GameplayStatics.PlaySound2D` "/Game/MilitaryWeapSilver/Sound/Rifle/Wavs/Rifle_Reload01.Rifle_Reload01" 1.0 1.0 0.0 null null)
    (`KismetSystemLibrary.Delay` 1.5)
    (`GameplayStatics.PlaySound2D` "/Game/MilitaryWeapSilver/Sound/Rifle/Wavs/Rifle_Reload02.Rifle_Reload02" 1.0 1.0 0.0 null null)
    (if (> (`.MaxAmmo_31_F054BC5D47269EC4CA695EBDF480892B` (break `/Game/Itens/PickUps/ItemType` (`self.ItemInfo`))) 0)
      (set `self.NeededAmmo` (- _clipsize _currentammo))
      (if (<= _maxammo _neededammo)
        (setmembers `/Game/Itens/PickUps/ItemType` :`StructRef` _iteminfo :`CurrentAmmo` (+ _currentammo_2 _maxammo_2))
        (setmembers `/Game/Itens/PickUps/ItemType` :`StructRef` _iteminfo :`MaxAmmo` 0)
        (else
          (setmembers `/Game/Itens/PickUps/ItemType` :`StructRef` _iteminfo :`MaxAmmo` (- _maxammo _neededammo))
          (setmembers `/Game/Itens/PickUps/ItemType` :`StructRef` _iteminfo :`CurrentAmmo` (`.ClipSize_40_72C2966E40FC4674620B56A55A8AC1F1` (break `/Game/Itens/PickUps/ItemType` (`self.ItemInfo`)))))))))

(fn `On/OffVisibility/CustomDepth`
  (params (bNewVisibility :type Boolean) (bValue :type Boolean))
  (`SceneComponent.SetVisibility` (`self.Widget`) bNewVisibility false)
  (`PrimitiveComponent.SetRenderCustomDepth` (`self.SkeletalMesh`) bValue))

(fn `UserConstructionScript`
  (bind (_iteminfo_itemtype _iteminfo_itemclass _iteminfo_clipsize _iteminfo_currentammo _iteminfo_maxammo _iteminfo_damage _iteminfo_itemimage _iteminfo_equipsocketname _iteminfo_unequipsocketname) (break `/Game/Itens/PickUps/ItemType` (`self.ItemInfo`)))
  (set `self.ItemInfo` (make `/Game/Itens/PickUps/ItemType` _iteminfo_itemtype (`GameplayStatics.GetObjectClass` self) _iteminfo_clipsize _iteminfo_currentammo _iteminfo_maxammo _iteminfo_damage _iteminfo_itemimage _iteminfo_equipsocketname _iteminfo_unequipsocketname)))