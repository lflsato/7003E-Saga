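; SimpleAI is a monster enemy that wanders, chases characters it sees and dies to magic projectiles.
; Tick starts moves to random reachable points while idle; PawnSensing starts an endless AIMoveTo chase loop that keeps IsMoving set.
; Projectile overlaps spawn an explosion, reduce Health and destroy the projectile.
; Death awards experience through ThirdPersonGameMode, handling level-ups with a doubled threshold and LevelUP widget, then destroys the monster.
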(event `self.ReceiveBeginPlay`)

(event `self.ReceiveActorBeginOverlap`
  (params (OtherActor :type "Actor Object Reference"))
  (bind _asmagic_projetile (cast `/Game/Kalebe/Blueprints/MagicProjetile` OtherActor))
  (`GameplayStatics.SpawnEmitterAtLocation` "/Game/StarterContent/Particles/P_Explosion.P_Explosion" (`self.K2_GetActorLocation` _asmagic_projetile))
  (set `self.Health` (- (`self.Health`) 50.0))
  (if (<= (`self.Health`) 0.0)
    (`self.Death`)
    (`self.K2_DestroyActor` _asmagic_projetile)
    (else
      (`self.K2_DestroyActor` _asmagic_projetile))))

(event `self.PawnSensing.OnSeePawn`
  (params (Pawn :type "Pawn Object Reference"))
  (bind _ascharacter (cast `Character` Pawn))
  (set `self.isMoving` true)
  (`|AIMoveTo` self (0.0 0.0 0.0) _ascharacter :!label _label
    (:`OnSuccess`
      _)
    (:`OnFail`
      _))
  (`KismetSystemLibrary.Delay` 0.5)
  (goto _label))

(event `self.ReceiveTick`
  (params (DeltaSeconds :type "Float (single-precision)"))
  (`KismetSystemLibrary.Delay` 2.0)
  (if (not (`self.isMoving`))
    (set `self.isMoving` true)
    (`|AIMoveTo` self (`NavigationSystemV1.K2_GetRandomReachablePointInRadius` (`self.K2_GetActorLocation`) 1000.0 null null) null
      (:`OnSuccess`
        _)
      (:`OnFail`
        _))
    (set `self.isMoving` false)))

(fn `Death`
  (bind _asthird_person_game_mode (cast `/Game/UI/ThirdPersonGameMode` (`GameplayStatics.GetGameMode`)))
  (bind _output_get (set `/Game/UI/ThirdPersonGameMode.Experience` (+ (`/Game/UI/ThirdPersonGameMode.Experience` _asthird_person_game_mode) 1) _asthird_person_game_mode))
  (if (>= _output_get (`/Game/UI/ThirdPersonGameMode.MaxExperience` _asthird_person_game_mode))
    ;[1 1 1] Subiu de level
    (set `/Game/UI/ThirdPersonGameMode.Level` (+ (`/Game/UI/ThirdPersonGameMode.Level` _asthird_person_game_mode) 1) _asthird_person_game_mode)
    (set `/Game/UI/ThirdPersonGameMode.Experience` 0 _asthird_person_game_mode)
    (set `/Game/UI/ThirdPersonGameMode.MaxExperience` (* (`/Game/UI/ThirdPersonGameMode.MaxExperience` _asthird_person_game_mode) 2) _asthird_person_game_mode)
    (bind _returnvalue (`|CreateWidget` "/Game/UI/HUD/LevelUP.LevelUP_C"))
    (`UserWidget.AddToViewport` _returnvalue 0))
  (`self.K2_DestroyActor`)
  (return))

(fn `TakeDamage`
  (`GameplayStatics.SpawnEmitterAtLocation` "/Game/StarterContent/Particles/P_Explosion.P_Explosion" (`self.K2_GetActorLocation`)))

(fn `UserConstructionScript`)