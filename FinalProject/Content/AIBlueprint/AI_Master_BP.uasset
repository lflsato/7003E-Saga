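; Base AI enemy that wanders, chases seen characters and grants experience when killed.
; Tick with a Delay picks random reachable points until PawnSensing sees a Character, then AIMoveTo re-issues every half second.
; MagicProjetile overlaps deal fixed damage, while ITakeDamage applies bullet damage with instant-kill headshots; health links to an AI_HUD widget.
; Death updates ThirdPersonGameMode experience, handling level-ups with a doubled threshold and LevelUP widget, then destroys the actor.
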(event `self.ReceiveActorBeginOverlap`
  (params (OtherActor :type "Actor Object Reference"))
  ;[1 1 1] Magic hit system
  (bind _asmagic_projetile (cast `/Game/Personagens/MagicProjetile` OtherActor))
  (`GameplayStatics.SpawnEmitterAtLocation` "/Game/StarterContent/Particles/P_Explosion.P_Explosion" (`self.K2_GetActorLocation` _asmagic_projetile))
  (set `self.CurrentHealth` (- (`self.CurrentHealth`) 100.0))
  (if (<= (`self.CurrentHealth`) 0.0)
    (`self.Death`)
    (`self.K2_DestroyActor` _asmagic_projetile)
    (else
      (`self.K2_DestroyActor` _asmagic_projetile))))

(event `self.ReceiveBeginPlay`
  ;[1 1 1] Initiate health AI system
  (set `self.CurrentHealth` (`self.MaxHealth`))
  (bind _asai_hud (cast `/Game/AIBlueprint/AI_HUD` (`WidgetComponent.GetUserWidgetObject` (`self.Widget`))))
  (set `/Game/AIBlueprint/AI_HUD.Owner` self _asai_hud))

(event `/Game/AIBlueprint/TakeDamage.ITakeDamage`
  (params (BoneName :type Name) (Damage :type "Float (single-precision)"))
  (bind _currenthealth (`self.CurrentHealth`))
  ;[1 1 1] Bullet hit system
  (if (== BoneName "Head")
    (set `self.CurrentHealth` 0.0)
    (else
      (set `self.CurrentHealth` (- _currenthealth Damage))))
  (if (<= _currenthealth 0.0)
    (`GameplayStatics.SpawnEmitterAtLocation` "/Game/StarterContent/Particles/P_Explosion.P_Explosion" (`self.K2_GetActorLocation`))
    (`self.Death`)
    (`self.K2_DestroyActor`)))

(event `self.PawnSensing.OnSeePawn`
  (params (Pawn :type "Pawn Object Reference"))
  ;[1 1 1] Follow main character by see it
  (bind _ascharacter (cast `Character` Pawn))
  (set `self.isMoving` true)
  (`|AIMoveTo` self (0.0 0.0 0.0) _ascharacter :!label _label
    (:`OnSuccess`
      _)
    (:`OnFail`
      _))
  (`KismetSystemLibrary.Delay` 0.5)
  (goto _label))

(event `self.ReceiveTick`
  (params (DeltaSeconds :type "Float (single-precision)"))
  ;[1 1 1] Enemy walk to a random position when is not alert
  (`KismetSystemLibrary.Delay` 2.0)
  (if (not (`self.isMoving`))
    (set `self.isMoving` true)
    (`|AIMoveTo` self (`NavigationSystemV1.K2_GetRandomReachablePointInRadius` (`self.K2_GetActorLocation`) 1000.0 null null) null
      (:`OnSuccess`
        _)
      (:`OnFail`
        _))
    (set `self.isMoving` false)))

(fn `Death`
  (bind _asthird_person_game_mode (cast `/Game/ThirdPersonBP/ThirdPersonGameMode` (`GameplayStatics.GetGameMode`)))
  (bind _output_get (set `/Game/ThirdPersonBP/ThirdPersonGameMode.Experience` (+ (`/Game/ThirdPersonBP/ThirdPersonGameMode.Experience` _asthird_person_game_mode) 1) _asthird_person_game_mode))
  (if (>= _output_get (`/Game/ThirdPersonBP/ThirdPersonGameMode.MaxExperience` _asthird_person_game_mode))
    ;[1 1 1] Subiu de level
    (set `/Game/ThirdPersonBP/ThirdPersonGameMode.Level` (+ (`/Game/ThirdPersonBP/ThirdPersonGameMode.Level` _asthird_person_game_mode) 1) _asthird_person_game_mode)
    (set `/Game/ThirdPersonBP/ThirdPersonGameMode.Experience` 0 _asthird_person_game_mode)
    (set `/Game/ThirdPersonBP/ThirdPersonGameMode.MaxExperience` (* (`/Game/ThirdPersonBP/ThirdPersonGameMode.MaxExperience` _asthird_person_game_mode) 2) _asthird_person_game_mode)
    (bind _returnvalue (`|CreateWidget` "/Game/HUD/LevelUP.LevelUP_C"))
    (`UserWidget.AddToViewport` _returnvalue 0))
  (`self.K2_DestroyActor`))

(fn `UserConstructionScript`)